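; Generated dynamic mesh actor that chains Geometry Script operations when its mesh rebuilds, apparently as a test of the nodes.
; OnRebuildGeneratedMesh appends revolve, spiral revolve and swept polygons, then applies offset, Perlin noise, mirror and union boolean before a collision-from-mesh call.
; Only the revolve receives polygon vertices; the other two shapes, the boolean's tool mesh and the collision's target component are left unset.
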(event EventBeginPlay)

(event Collision|EventActorBeginOverlap
  (params (OtherActor :type Actor%20Object%20Reference)))

(event EventTick
  (params (DeltaSeconds :type Float%20%28single-precision%29)))

(event Events|EventOnRebuildGeneratedMesh
  (params (TargetMesh :type Dynamic%20Mesh%20Object%20Reference))
  (bind _returnvalue (Class|GeometryScriptLibraryMeshPrimitiveFunctions|AppendRevolvePolygon :TargetMesh TargetMesh :PolygonVertices (Utilities|Array|MakeArray "" "(X=10.000000,Y=0.000000)" "(X=10.000000,Y=10.000000)" "(X=0.000000,Y=10.000000)") :RevolveOptions (Utilities|Struct|MakeGeometryScriptRevolveOptions 3.6e+02 0.0) :Steps 20 :Debug 0))
  (bind _returnvalue_2 (Class|GeometryScriptLibraryMeshPrimitiveFunctions|AppendSpiralRevolvePolygon :TargetMesh _returnvalue :Debug 0))
  (bind _returnvalue_3 (Class|GeometryScriptLibraryMeshPrimitiveFunctions|AppendSimpleSweptPolygon :TargetMesh _returnvalue_2 :Debug 0))
  (bind _returnvalue_4 (Class|GeometryScriptLibraryMeshModelingFunctions|ApplyMeshOffset _returnvalue_3 (Utilities|Struct|MakeGeometryScriptMeshOffsetOptions 1.0 false) 0))
  (bind _returnvalue_5 (Class|GeometryScriptLibraryMeshDeformFunctions|ApplyPerlinNoisetoMesh _returnvalue_4 (Utilities|Struct|MakeGeometryScriptPerlinNoiseOptions (Utilities|Struct|MakeGeometryScriptPerlinNoiseLayerOptions 5.0 0.25 "0.000000,0.000000,0.000000") true) 0))
  (bind _returnvalue_6 (Class|GeometryScriptLibraryMeshBooleanFunctions|ApplyMeshMirror _returnvalue_5 (Variables|Default|GetMirror%20Frame) (Utilities|Struct|MakeGeometryScriptMeshMirrorOptions true false true) 0))
  (bind _returnvalue_7 (GeometryScript|Booleans|ApplyMeshBoolean :TargetMesh _returnvalue_6 :Operation "Union" :Options (Utilities|Struct|MakeGeometryScriptMeshBooleanOptions true true 0.01) :Debug 0))
  (Class|GeometryScriptLibraryCollisionFunctions|SetDynamicMeshCollisionfromMesh _returnvalue_7 0 (Utilities|Struct|MakeGeometryScriptCollisionfromMeshOptions true "MinVolumeShapes") 0))

(fn ConstructionScript)